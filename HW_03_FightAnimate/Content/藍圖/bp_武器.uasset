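; Weapon Blueprint (bp_武器) that handles automatic firing and ammo for the player character, BP_玩家控制.
; Holding the 開槍 input, unless reloading or sprinting at press time, runs a Delay-paced loop spawning Bp_子彈 with weapon damage and a muzzle flash at the mesh socket until release or empty magazine.
; 換彈夾 refills the magazine from reserve ammo; 補充子彈 adds one magazine's worth to the reserve, clamped to its limit.
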(event Custom|換彈夾
  ;[1 1 1] 換彈夾
  (Variables|Default|Set要補充的子彈數量 (- (Variables|Default|Get彈夾尺寸) (Variables|Default|Get目前子彈數量)))
  (if (>= (Variables|Default|Get子彈總數) (Variables|Default|Get要補充的子彈數量))
    _
    (else
      (Variables|Default|Set要補充的子彈數量 (Variables|Default|Get子彈總數))))
  (Variables|Default|Set目前子彈數量 (+ (Variables|Default|Get目前子彈數量) (Variables|Default|Get要補充的子彈數量)))
  (Variables|Default|Set子彈總數 (- (Variables|Default|Get子彈總數) (Variables|Default|Get要補充的子彈數量))))

(event Custom|補充子彈
  (bind _output_get (Variables|Default|Set子彈總數 (+ (Variables|Default|Get子彈總數) (Variables|Default|Get彈夾尺寸))))
  (Variables|Default|Set子彈總數 (Math|Integer|Clamp(Integer) _output_get 0 (Variables|Default|Get子彈上限))))

(event EventBeginPlay
  ;[0.2865 0.731 1] 取得玩家資訊
  (bind _asbp_玩家控制 (Utilities|Casting|CastToBP_玩家控制 (Game|GetPlayerCharacter 0)))
  (Variables|Default|Set玩家控制 _asbp_玩家控制))

(event Input|ActionEvents|InputAction開槍
  (params (Key :type Key%20Structure :default "None"))
  (bind _武器 (Variables|Default|Get武器))
  (bind _玩家控制 (Variables|Default|Get玩家控制))
  (bind _returnvalue (Transformation|GetSocketRotation _武器 "None"))
  ;[1 1 1] 開槍
  (:Pressed
    (if (and (not (Variables|/Game/藍圖/BP_玩家控制.BP_玩家控制_C|Get換彈夾 _玩家控制)) (not (Variables|/Game/藍圖/BP_玩家控制.BP_玩家控制_C|Get衝刺 _玩家控制)))
      (Variables|Default|Set開槍中 true)
      (if (and (> (Variables|Default|Get目前子彈數量) 0) (Variables|Default|Get開槍中)) :!label _label
        (bind _returnvalue_2 (Game|SpawnActorfromClass "/Game/藍圖/bp_子彈.bp_子彈_C" (Transformation|GetSocketTransform (Variables|Default|Get武器) "子彈插槽" "RTS_World") "Undefined" 0 0))
        (Variables|/Game/藍圖/bp_子彈.bp_子彈_C|Set目前武器傷害 _returnvalue_2 (Variables|Default|Get武器傷害))
        (Effects|SpawnEmitteratLocation "/Game/InfinityBladeEffects/Effects/FX_Monsters/FX_Monster_Gruntling/Master/P_BackPack_MuzzleFlash.P_BackPack_MuzzleFlash" (Transformation|GetSocketLocation _武器 "子彈插槽") (Math|Rotator|MakeRotator (+ (.roll _returnvalue) 9e+01) (.pitch _returnvalue) (+ (.yaw _returnvalue) 9e+01)) "0.100000,0.100000,0.100000")
        (Variables|Default|Set目前子彈數量 (- (Variables|Default|Get目前子彈數量) 1))
        (Utilities|FlowControl|Delay (Variables|Default|Get開槍間隔))
        (goto _label))))
  (:Released
    (Variables|Default|Set開槍中 false)))

(fn ConstructionScript)